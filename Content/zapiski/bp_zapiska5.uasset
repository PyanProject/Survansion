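; Readable note pickup (zapiska 5) that the player toggles open and closed with the E interaction event.
; Each press plays a pickup sound and sets IsZapiska2 on the first-person character, then a FlipFlop alternates states.
; Opening shows the Zapiska5 widget, disables the camera and flashlight pick flags, and ignores look and move input; closing removes the widget and restores them.
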(event EventPressEInteraction
  (params (HitActor :type Object%20Object%20Reference))
  (bind _returnvalue (Game|GetPlayerController 0))
  (bind _asbp_first_person_character (Utilities|Casting|CastToBP_FirstPersonCharacter (Game|GetPlayerCharacter 0)))
  (Variables|/Game/FirstPerson/Blueprints/BP_FirstPersonCharacter.BP_FirstPersonCharacter_C|SetIsZapiska2 _asbp_first_person_character true)
  (Audio|PlaySound2D "/Game/StarterContent/Audio/Game_Sounds/Sounds/TakeZapiska.TakeZapiska" 1.0 1.0 0.0 0 0)
  (Utilities|FlowControl|FlipFlop
    (:A
      (Variables|/Game/FirstPerson/Blueprints/BP_FirstPersonCharacter.BP_FirstPersonCharacter_C|SetPickCamera _asbp_first_person_character false)
      (Variables|/Game/FirstPerson/Blueprints/BP_FirstPersonCharacter.BP_FirstPersonCharacter_C|SetPickFlash _asbp_first_person_character false)
      (bind _returnvalue_2 (Game|ConstructObjectfromClass "/Game/UI/zapiski_widget/zapiska5.zapiska5_C"))
      (UserInterface|Viewport|AddtoViewport _returnvalue_2 0)
      (Input|SetIgnoreLookInput _returnvalue true)
      (Input|SetIgnoreMoveInput _returnvalue true))
    (:B
      (Variables|/Game/FirstPerson/Blueprints/BP_FirstPersonCharacter.BP_FirstPersonCharacter_C|SetPickCamera _asbp_first_person_character true)
      (Variables|/Game/FirstPerson/Blueprints/BP_FirstPersonCharacter.BP_FirstPersonCharacter_C|SetPickFlash _asbp_first_person_character true)
      (Widget|RemovefromParent _returnvalue_2)
      (Input|SetIgnoreLookInput _returnvalue false)
      (Input|SetIgnoreMoveInput _returnvalue false))))

(fn ConstructionScript)