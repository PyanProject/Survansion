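; FlashBP is a flashlight pickup that the player collects through an interaction.
; BeginPlay creates a Press_E prompt widget, which the Interaction event shows on screen for one second.
; PressEInteraction casts the player to BP_FirstPersonCharacter, sets its PickFlash flag and a Russian "flashlight received" notice, then removes the prompt and destroys the actor.
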(event EventBeginPlay
  (bind _returnvalue (UserInterface|CreateWidget "/Game/UI/ObjectiveMarkers/Press_E.Press_E_C"))
  (Variables|Default|SetWidget _returnvalue))

(event EventInteraction
  (bind _widget (Variables|Default|GetWidget))
  (UserInterface|Viewport|AddtoViewport _widget 0)
  (Utilities|FlowControl|Delay 1.0)
  (Widget|RemovefromParent _widget))

(event EventPressEInteraction
  (params (HitActor :type Object%20Object%20Reference))
  (bind _asbp_first_person_character (Utilities|Casting|CastToBP_FirstPersonCharacter (Game|GetPlayerCharacter 0)))
  (Default|SetNotice _asbp_first_person_character "Получен фонарик")
  (Variables|/Game/FirstPerson/Blueprints/BP_FirstPersonCharacter.BP_FirstPersonCharacter_C|SetPickFlash _asbp_first_person_character true)
  (Widget|RemovefromParent (Variables|Default|GetWidget))
  (Actor|DestroyActor))

(fn ConstructionScript)