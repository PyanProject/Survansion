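; Player character Blueprint with basic movement, look controls and a toggleable flashlight.
; Axis inputs drive movement and controller yaw and pitch, and BeginPlay lowers the walk speed.
; Once PickFlash is true, the flash action alternates the SpotLight on and off through a FlipFlop, with a sound for each state.
; Tick aligns the SpotLight to the control rotation so the beam follows the view.
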(event EventBeginPlay
  (Variables|/Script/Engine.CharacterMovementComponent|SetMaxWalkSpeed (Variables|Character|GetCharacterMovement) 2.5e+02))

(event EventTick
  (params (DeltaSeconds :type Float%20%28single-precision%29))
  (Utilities|FlowControl|Sequence
    (:then_0
      (Transformation|SetWorldRotation (Variables|Default|GetSpotLight) (Pawn|GetControlRotation :!class /Script/Engine.Pawn) false false))))

(event Input|ActionEvents|InputActionflash
  (params (Key :type Key%20Structure :default "None"))
  (bind _spotlight (Variables|Default|GetSpotLight))
  (bind _returnvalue (Transformation|GetWorldLocation _spotlight))
  (:Pressed
    (if (Variables|Default|GetPickFlash)
      (Utilities|FlowControl|FlipFlop
        (:A
          (Audio|PlaySoundatLocation "/Game/Phonarik/FlashOn.FlashOn" _returnvalue "0, 0, 0" 0.5 1.0 0.0 0 0 0 0)
          (Rendering|SetVisibility _spotlight true false))
        (:B
          (Audio|PlaySoundatLocation "/Game/Phonarik/FlashOff.FlashOff" _returnvalue "0, 0, 0" 0.3 1.0 0.0 0 0 0 0)
          (Rendering|SetVisibility _spotlight false false))))))

(event Input|AxisEvents|InputAxisforwardback
  (params (AxisValue :type Float%20%28single-precision%29))
  ;[1 1 1] Movement
  (Pawn|Input|AddMovementInput (Transformation|GetActorForwardVector) AxisValue false))

(event Input|AxisEvents|InputAxisleftright
  (params (AxisValue :type Float%20%28single-precision%29))
  ;[1 1 1] Movement
  (Pawn|Input|AddMovementInput (Math|Vector|GetRightVector (Pawn|GetControlRotation :!class /Script/Engine.Pawn)) AxisValue false))

(event Input|AxisEvents|InputAxisverticale
  (params (AxisValue :type Float%20%28single-precision%29))
  ;[1 1 1] Movement
  (Pawn|Input|AddControllerYawInput (* AxisValue 1.0)))

(event Input|AxisEvents|InputAxishorizontale
  (params (AxisValue :type Float%20%28single-precision%29))
  ;[1 1 1] Movement
  (Pawn|Input|AddControllerPitchInput (* AxisValue -1.0)))

(fn ConstructionScript)