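; BP_key3 is a key pickup that unlocks its matching door for the first-person player.
; Interaction shows a Press_E prompt widget, created on BeginPlay, for one second.
; PressEInteraction looks up the hit actor in the character's KeyInventory map, sets that value to true in its Doors map, then removes the prompt and destroys the key.
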(event EventBeginPlay
  (bind _returnvalue (UserInterface|CreateWidget "/Game/UI/ObjectiveMarkers/Press_E.Press_E_C"))
  (Variables|Default|SetWidget _returnvalue))

(event EventInteraction
  (bind _widget (Variables|Default|GetWidget))
  (UserInterface|Viewport|AddtoViewport _widget 0)
  (Utilities|FlowControl|Delay 1.0)
  (Widget|RemovefromParent _widget))

(event EventPressEInteraction
  (params (HitActor :type Object%20Object%20Reference))
  (bind _asbp_first_person_character (Utilities|Casting|CastToBP_FirstPersonCharacter (Game|GetPlayerCharacter 0)))
  (bind _asactor (Utilities|Casting|CastToActor HitActor))
  (Utilities|Map|Add (Variables|/Game/FirstPerson/Blueprints/BP_FirstPersonCharacter.BP_FirstPersonCharacter_C|GetDoors _asbp_first_person_character) (.Value (Utilities|Map|Find (Variables|/Game/FirstPerson/Blueprints/BP_FirstPersonCharacter.BP_FirstPersonCharacter_C|GetKeyInventory _asbp_first_person_character) _asactor)) true)
  (Widget|RemovefromParent (Variables|Default|GetWidget))
  (Actor|DestroyActor))

(fn ConstructionScript)