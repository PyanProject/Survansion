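; A crumpled paper garbage prop that makes noise when it takes a hard hit.
; When the hit impulse on its mesh exceeds a threshold, it reports an AI noise event at the mesh location and plays its audio, which is silenced on BeginPlay.
; It also writes that location as the last noise location into the MainAnimBP on the player character's Leg mesh.
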(event OnComponentHit(bbf2df363493_a_crumpled_paper__3_high_poly)
  (params (HitComponent :type Primitive%20Component%20Object%20Reference) (OtherActor :type Actor%20Object%20Reference) (OtherComp :type Primitive%20Component%20Object%20Reference) (NormalImpulse :type Vector :default "0, 0, 0") (Hit :type Hit%20Result%20Structure%20%28by%20ref%29))
  (bind _bbf2df363493_a_crumpled_paper__3_high_poly (Variables|Default|Getbbf2df363493_a_crumpled_paper__3_high_poly))
  (bind _returnvalue (Transformation|GetWorldLocation _bbf2df363493_a_crumpled_paper__3_high_poly))
  (Math|Float|CompareFloat (Math|Vector|VectorLength NormalImpulse) 6e+03
    (:>
      (Class|AISenseHearing|ReportNoiseEvent _returnvalue 1.0 self 3e+03 "None")
      (Audio|Components|Audio|Play (Variables|Default|GetAudio) 0.0)
      (bind _asbp_first_person_character (Utilities|Casting|CastToBP_FirstPersonCharacter (Game|GetPlayerCharacter 0)))
      (bind _output_get (Variables|Default|SetAs%20BP%20First%20Person%20Character _asbp_first_person_character))
      (bind _asmain_anim_bp (Utilities|Casting|CastToMainAnimBP (Components|SkeletalMesh|GetAnimInstance (Variables|/Game/FirstPerson/Blueprints/BP_FirstPersonCharacter.BP_FirstPersonCharacter_C|GetLeg _output_get))))
      (Variables|/Game/Characters/Mannequins/Animations/Custom/Blueprints/MainAnimBP.MainAnimBP_C|SetLastNoiseLocation _asmain_anim_bp _returnvalue))))

(event EventBeginPlay
  (Audio|Components|Audio|Stop (Variables|Default|GetAudio)))

(fn ConstructionScript)