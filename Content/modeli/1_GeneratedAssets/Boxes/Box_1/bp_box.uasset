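; Box prop Blueprint that makes a sound and alerts AI hearing when it takes a hard impact.
; Its mesh's hit event prints the normal impulse magnitude and, above a fixed threshold, reports a ranged noise event at the box's location and plays the Audio component.
; BeginPlay stops the audio so it starts silent; a first-person character cast and comparison are left unconnected.
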(event OnComponentHit(e6ed038aa53d_Old_boxes_min_mesh)
  (params (HitComponent :type Primitive%20Component%20Object%20Reference) (OtherActor :type Actor%20Object%20Reference) (OtherComp :type Primitive%20Component%20Object%20Reference) (NormalImpulse :type Vector :default "0, 0, 0") (Hit :type Hit%20Result%20Structure%20%28by%20ref%29))
  (bind _returnvalue (Math|Vector|VectorLength NormalImpulse))
  (bind _self self)
  (Development|PrintString (Utilities|String|ToString(Float) _returnvalue))
  (Math|Float|CompareFloat _returnvalue 6e+03
    (:>
      (Class|AISenseHearing|ReportNoiseEvent (Transformation|GetActorLocation _self) 1.0 _self 3e+03 "None")
      (Audio|Components|Audio|Play (Variables|Default|GetAudio) 0.0))))

(event EventBeginPlay
  (Audio|Components|Audio|Stop (Variables|Default|GetAudio)))

(fn ConstructionScript)