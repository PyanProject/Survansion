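; Point light Blueprint that applies its intensity, radius and main color at BeginPlay and exposes on, off and ghost-effect events.
; LightOn and LightOff fade intensity through a Timeline, except for the Signal type, which swaps between main and secondary colors.
; GhostLight runs a FlipFlop and Delay flicker loop for several seconds, holds dark red, then restores a warm color at zero intensity.
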(event Custom|LightOff
  (switch string (Variables|Default|GetIdx)
    (:Default
      (bind _alpha (Timeline|Timeline ReverseFromEnd)
        (:Update
          (Rendering|Components|Light|SetIntensity (Variables|Default|GetPointLight) (Math|Float|Lerp 0.0 (Variables|Default|GetIntensity) _alpha)))))
    (:Signal
      (Rendering|Components|Light|SetLightColor (Variables|Default|GetPointLight) (Variables|Default|GetSecondLightColor) true))))

(event Custom|LightOn
  (switch string (Variables|Default|GetIdx)
    (:Default
      (bind _alpha (Timeline|Timeline PlayFromStart)
        (:Update
          (Rendering|Components|Light|SetIntensity (Variables|Default|GetPointLight) (Math|Float|Lerp 0.0 (Variables|Default|GetIntensity) _alpha)))))
    (:Signal
      (Rendering|Components|Light|SetLightColor (Variables|Default|GetPointLight) (Variables|Default|GetMainLightColor) true))))

(event Custom|GhostLight
  (bind _pointlight (Variables|Default|GetPointLight))
  (bind _pointlight_2 (Variables|Default|GetPointLight))
  (Variables|Default|SetCondition true)
  (Utilities|FlowControl|Sequence
    (:then_0
      (if (Variables|Default|GetCondition) :!label _label
        (Utilities|FlowControl|FlipFlop
          (:A
            (Rendering|Components|Light|SetIntensity _pointlight 5.0)
            (Utilities|FlowControl|Delay 0.1)
            (goto _label))
          (:B
            (Rendering|Components|Light|SetIntensity _pointlight 0.0)
            (Utilities|FlowControl|Delay 0.15)
            (goto _label)))))
    (:then_1
      (Utilities|FlowControl|Delay 9.0)
      (Variables|Default|SetCondition false)
      (Rendering|Components|Light|SetIntensity (Variables|Default|GetPointLight) 6.0)
      (Rendering|Components|Light|SetLightColor _pointlight_2 "(R=0.223958,G=0.000000,B=0.000000,A=1.000000)" true)
      (Utilities|FlowControl|Delay 4.0)
      (Rendering|Components|Light|SetLightColor _pointlight_2 "(R=1.000000,G=0.879623,B=0.590619,A=1.000000)" true)
      (Rendering|Components|Light|SetIntensity _pointlight_2 0.0))))

(event EventBeginPlay
  (Rendering|Components|Light|SetIntensity (Variables|Default|GetPointLight) (Variables|Default|GetIntensity))
  (Rendering|Lighting|SetAttenuationRadius (Variables|Default|GetPointLight) (Variables|Default|GetRadius))
  (Rendering|Components|Light|SetLightColor (Variables|Default|GetPointLight) (Variables|Default|GetMainLightColor) true))

(fn ConstructionScript)