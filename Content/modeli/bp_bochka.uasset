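; Plastic drum prop (bochka) that makes noise when the player character knocks into it hard.
; GasDropCue audio is stopped on BeginPlay, and component hits on the drum mesh print their impulse magnitude to screen.
; When the hitting actor is the player and the impulse exceeds a threshold, it reports a ranged AI noise event at its location and plays the cue.
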(event OnComponentHit(S_Dirty_Plastic_Drum_uiujbcxva_lod0_Var1)
  (params (HitComponent :type Primitive%20Component%20Object%20Reference) (OtherActor :type Actor%20Object%20Reference) (OtherComp :type Primitive%20Component%20Object%20Reference) (NormalImpulse :type Vector :default "0, 0, 0") (Hit :type Hit%20Result%20Structure%20%28by%20ref%29))
  (bind _returnvalue (Math|Vector|VectorLength NormalImpulse))
  (bind _asbp_first_person_character (Utilities|Casting|CastToBP_FirstPersonCharacter (Game|GetPlayerCharacter 0)))
  (Development|PrintString (Utilities|String|ToString(Float) _returnvalue))
  (if (== OtherActor _asbp_first_person_character)
    (Math|Float|CompareFloat _returnvalue 5e+02
      (:>
        (Class|AISenseHearing|ReportNoiseEvent (Transformation|GetActorLocation) 1.0 self 3e+03 "None")
        (Audio|Components|Audio|Play (Variables|Default|Getgas_drop_Cue) 0.0)))))

(event EventBeginPlay
  (Audio|Components|Audio|Stop (Variables|Default|Getgas_drop_Cue)))

(fn ConstructionScript)