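; OldCamewra_BP is a pickup actor for an old camera that the player collects with a press-E interaction.
; It creates a Press_E widget at BeginPlay and shows it for half a second whenever Interaction fires.
; PressEInteraction sets PickCamera on BP_FirstPersonCharacter, posts a Russian "camera received" notice, removes the prompt and destroys the actor.
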(event EventBeginPlay
  (bind _returnvalue (UserInterface|CreateWidget "/Game/UI/ObjectiveMarkers/Press_E.Press_E_C"))
  (Variables|Default|SetWidget _returnvalue))

(event EventInteraction
  (UserInterface|Viewport|AddtoViewport (Variables|Default|GetWidget) 0)
  (Utilities|FlowControl|Delay 0.5)
  (Widget|RemovefromParent (Variables|Default|GetWidget)))

(event EventPressEInteraction
  (params (HitActor :type Object%20Object%20Reference))
  (bind _asbp_first_person_character (Utilities|Casting|CastToBP_FirstPersonCharacter (Game|GetPlayerCharacter 0)))
  (Default|SetNotice _asbp_first_person_character "Получена камера")
  (Variables|/Game/FirstPerson/Blueprints/BP_FirstPersonCharacter.BP_FirstPersonCharacter_C|SetPickCamera _asbp_first_person_character true)
  (Widget|RemovefromParent (Variables|Default|GetWidget))
  (Actor|DestroyActor))

(fn ConstructionScript)